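; BP_SoundMaster is an unfinished audio visualizer actor that sets a sound on its Audio component and records its duration at BeginPlay.
; PlayBackChange converts playback percent to seconds and loops over normalized Constant-Q values for channel 0, a pre-analyzed spectrum lookup, with an empty loop body.
; The playback-percent binding and the Sphere scaling driven by those values are disconnected, and the scale multiplier is zero.
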(event Custom|PlayBackChange
  (params (PlayingSoundWave :type Sound%20Wave%20Object%20Reference) (PlaybackPercent :type Float%20%28single-precision%29))
  (Variables|Default|SetPlayedTime (* PlaybackPercent (Variables|Default|GetDuration)))
  (for _array_element (Class|ConstantQNRT|GetNormalizedChannelConstantQatTime (Variables|Default|GetRef_Constant) (Variables|Default|GetPlayedTime))
    _))

(event EventBeginPlay
  (Audio|Components|Audio|SetSound (Variables|Default|GetAudio) (Variables|Default|GetSound))
  (Variables|Default|SetDuration (Variables|/Script/Engine.SoundBase|GetDuration (Variables|Default|GetSound))))

(fn ConstructionScript)