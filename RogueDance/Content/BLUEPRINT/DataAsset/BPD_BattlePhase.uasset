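; BPD_BattlePhase is a data-holding Blueprint that tracks the battle phase through attack, defense and transition flags.
; SetAttack and SetDefense each switch their phase on and the other off, while SetTransition sets the transition flag independently.
; SetPhase acts as a toggle, turning attack into defense and defense into attack, defaulting to attack when both inputs are false, then returns both flags.
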(fn SetAttack
  (Variables|Default|SetAttackPhase true)
  (Variables|Default|SetDefensePhase false)
  (return))

(fn SetDefense
  (Variables|Default|SetDefensePhase true)
  (Variables|Default|SetAttackPhase false)
  (return))

(fn SetTransition
  (params (TransitionOn? :type Boolean))
  (Variables|Default|SetTransitionPhase TransitionOn?))

(fn SetPhase
  (params (Attack :type Boolean) (Defense :type Boolean))
  (if Attack
    (Variables|Default|SetDefensePhase true)
    (Variables|Default|SetAttackPhase false)
    (return (Variables|Default|GetAttackPhase) (Variables|Default|GetDefensePhase))
    (elif Defense
      (Variables|Default|SetAttackPhase true)
      (Variables|Default|SetDefensePhase false)
      (return (Variables|Default|GetAttackPhase) (Variables|Default|GetDefensePhase))
      (elif (and (== Attack false) (== Defense false))
        (Variables|Default|SetAttackPhase true)
        (Variables|Default|SetDefensePhase false)
        (return (Variables|Default|GetAttackPhase) (Variables|Default|GetDefensePhase))))))