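; Flipbook-animated enemy bot for a rhythm-driven battle, timed to a Quartz clock.
; Bar quantization events, subscribed from Tick while WannaTop is set, switch idle, ready, attack and down flipbooks on hard-coded bars.
; Once released in DefensePhase, it lerps to BP_CypherLocation via a Timeline, snapping when close, and returns to its start in AttackPhase.
; The all-beat subscription never runs, and OnTheBeat has no visible subscription.
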(event Custom|On%20The%20Beat
  (params (ClockName :type Name) (QuantizationType :type EQuartzCommandQuantization%20Enum :default "Bar") (NumBars :type Integer) (Beat :type Integer) (BeatFraction :type Float%20%28single-precision%29))
  (|FirstAnimTestOnBeat NumBars NumBars NumBars))

(event Custom|Bar
  (params (ClockName :type Name) (QuantizationType :type EQuartzCommandQuantization%20Enum :default "Bar") (NumBars :type Integer) (Beat :type Integer) (BeatFraction :type Float%20%28single-precision%29))
  (bind _botflipbook (Variables|Default|GetBotFlipBook))
  (if (== NumBars 1)
    (Components|Timeline|SetPlayRate _botflipbook (Variables|Default|GetPlayRateModifier))
    (Sprite|SetFlipbook _botflipbook (Variables|Animation|GetIdleFlipbook))
    (Transformation|SetActorRotation "0.000000,180.000000,0.000000")
    (elif (Variables|/Game/BLUEPRINT/DataAsset/BPD_BattlePhase.BPD_BattlePhase_C|GetDefensePhase (Variables|Default|GetBattlePhase))
      (if (== NumBars 2)
        (Variables|Default|SetCanMoveAtStart true))
      (if (or (== NumBars 8) (== NumBars 16))
        (Sprite|SetFlipbook (Variables|Default|GetBotFlipBook) (Variables|Animation|GetReadyTopFlipBook))
        (elif (== NumBars 9)
          (Sprite|SetFlipbook (Variables|Default|GetBotFlipBook) (Variables|Animation|GetTopAttackFlipbook))
          (elif (Math|Boolean|ORBoolean (== NumBars 19) (== NumBars 21) (== NumBars 23) (== NumBars 17))
            (Sprite|SetFlipbook (Variables|Default|GetBotFlipBook) (Variables|Animation|GetDownFlipBook_1))
            (Transformation|SetActorRotation "0.000000,180.000000,0.000000")))))))

(event Custom|OnAllBeat
  (params (ClockName :type Name) (QuantizationType :type EQuartzCommandQuantization%20Enum :default "Bar") (NumBars :type Integer) (Beat :type Integer) (BeatFraction :type Float%20%28single-precision%29))
  (|UpdateAllQuantizeEvent QuantizationType NumBars NumBars Beat Beat Beat Beat))

(event EventBeginPlay
  (bind _returnvalue (Actor|GetActorOfClass "/Game/BLUEPRINT/BP_CypherLocation.BP_CypherLocation_C"))
  (Variables|Default|SetCyperLocation (Transformation|GetActorLocation _returnvalue))
  (Variables|Default|SetCanMoveAtStart false)
  (Variables|Default|SetStartPos (Transformation|GetActorLocation)))

(event EventTick
  (params (DeltaSeconds :type Float%20%28single-precision%29))
  (Utilities|FlowControl|Sequence
    (:then_1
      (if (Variables|Default|GetWannaTop)
        (Class|QuartzClockHandle|SubscribetoQuantizationEvent (Variables|/Game/BLUEPRINT/DataAsset/BPD_Clock157.BPD_Clock157_C|GetClockTest (Variables|Default|GetRef%20Clock%20157)) "Bar" (delegate Custom|Bar))))
    (:then_2
      (if (Variables|Default|GetCanMoveAtStart)
        (if (Variables|/Game/BLUEPRINT/DataAsset/BPD_BattlePhase.BPD_BattlePhase_C|GetDefensePhase (Variables|Default|GetBattlePhase))
          (if (<= (Math|Vector|Distance(Vector) (Variables|Default|GetCyperLocation) (Transformation|GetActorLocation)) 2e+01)
            (Transformation|SetActorLocation (Variables|Default|GetCyperLocation) false false)
            (else
              (bind _newtrack_0 (Timeline|Timeline PlayFromStart)
                (:Update
                  (Transformation|SetActorLocation (Math|Vector|Lerp(Vector) (Transformation|GetActorLocation) (Variables|Default|GetCyperLocation) (* _newtrack_0 1.5)) false false)))))
          (elif (Variables|/Game/BLUEPRINT/DataAsset/BPD_BattlePhase.BPD_BattlePhase_C|GetAttackPhase (Variables|Default|GetBattlePhase))
            (Transformation|SetActorLocation (Variables|Default|GetStartPos) false false)))))))

(fn ConstructionScript
  (Variables|Default|SetSelfLocation (Transformation|GetActorTransform)))

(fn SetTopAnim
  (Variables|Default|SetPlayTop true))