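; Player controller Blueprint that sets up input and locks the view to the level camera.
; On BeginPlay it adds the MC_PlayerInput Enhanced Input mapping context and sets the view target to the BP_LevelCam found in the level.
; Tick repeats that camera lookup and view target switch every frame.
; A debug handler on IA_ChangeULT adds to CurrentHealth's Health each time the action triggers.
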(event Input|EnhancedActionEvents|EnhancedInputActionIA_ChangeULT
  (params (ActionValue :type Boolean) (ElapsedSeconds :type Float%20%28double-precision%29) (TriggeredSeconds :type Float%20%28double-precision%29) (InputAction :type Input%20Action%20Object%20Reference :default "/Game/INPUT/InputActions/IA_ChangeULT.IA_ChangeULT"))
  ;[0.15 0.15 0.15 0.5] DEBUG
  (:Triggered
    (Variables|/Game/BLUEPRINT/DataAsset/BP_Health.BP_Health_C|SetHealth (Variables|Default|GetCurrent_Health) (+ (Variables|/Game/BLUEPRINT/DataAsset/BP_Health.BP_Health_C|GetHealth (Variables|Default|GetCurrent_Health)) 10))))

(event EventBeginPlay
  (Utilities|FlowControl|Sequence
    (:then_0
      (Input|AddMappingContext (PlayerController|LocalPlayerSubsystems|GetEnhancedInputLocalPlayerSubsystem self) "/Game/INPUT/MC_PlayerInput.MC_PlayerInput" 0 "(bIgnoreAllPressedKeysUntilRelease=True,bForceImmediately=False,bNotifyUserSettings=False)"))
    (:then_1
      (bind _returnvalue (Actor|GetActorOfClass "/Game/BLUEPRINT/BP_LevelCam.BP_LevelCam_C"))
      (Game|Player|SetViewTargetwithBlend _returnvalue 0.0 "VTBlend_Linear" 0.0 false))))

(event EventTick
  (params (DeltaSeconds :type Float%20%28single-precision%29))
  (bind _returnvalue (Actor|GetActorOfClass "/Game/BLUEPRINT/BP_LevelCam.BP_LevelCam_C"))
  (Game|Player|SetViewTargetwithBlend _returnvalue 0.0 "VTBlend_Linear" 0.0 false))

(fn ConstructionScript)