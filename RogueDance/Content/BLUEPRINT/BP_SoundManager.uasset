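; Sound manager actor that keeps its Audio component on the same sound as its Analyser.
; The construction script copies the Analyser's sound into the Audio component and stores that sound's duration in a Duration variable.
; BeginPlay only prints the name of the assigned sound; overlap and tick events are unused.
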(event EventBeginPlay
  (Development|PrintString (Utilities|GetObjectName (Variables|/Script/Engine.AudioComponent|GetSound (Variables|Default|GetAudio)))))

(event Collision|EventActorBeginOverlap
  (params (OtherActor :type Actor%20Object%20Reference)))

(event EventTick
  (params (DeltaSeconds :type Float%20%28single-precision%29)))

(fn ConstructionScript
  (bind _analyser (Variables|Default|GetAnalyser))
  (bind _sound (Variables|/Script/AudioAnalyzer.AudioAnalyzerNRT|GetSound _analyser))
  (Audio|Components|Audio|SetSound (Variables|Default|GetAudio) _sound)
  (Variables|Default|SetDuration (Variables|/Script/Engine.SoundBase|GetDuration _sound)))