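; BP_PNJ_dialog is an NPC actor that shows an interaction prompt and steps through its dialogue lines.
; Its collision overlap with BP_Character reveals the prompt and creates a Dialog_UI widget; leaving hides both.
; EventDialogHappens passes NPCTxt to the widget, shows its panel, then advances TextIndex or removes the widget at the last index.
; A DoOnce gates each advance and is reset right afterwards.
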(event OnComponentBeginOverlap(collision)
  (params (OverlappedComponent :type Primitive%20Component%20Object%20Reference) (OtherActor :type Actor%20Object%20Reference) (OtherComp :type Primitive%20Component%20Object%20Reference) (OtherBodyIndex :type Integer) (bFromSweep :type Boolean) (SweepResult :type Hit%20Result%20Structure%20%28by%20ref%29))
  (Utilities|Casting|CastToBP_Character OtherActor)
  (Development|SetHiddeninGame (Variables|Default|GetInterraction_text) false false)
  (bind _returnvalue (UserInterface|CreateWidget "/Game/BLUEPRINT/Dialog_system/Dialog_UI.Dialog_UI_C"))
  (bind _output_get (Variables|Default|SetDialogUI _returnvalue))
  (UserInterface|Viewport|AddtoViewport _output_get 0))

(event OnComponentEndOverlap(collision)
  (params (OverlappedComponent :type Primitive%20Component%20Object%20Reference) (OtherActor :type Actor%20Object%20Reference) (OtherComp :type Primitive%20Component%20Object%20Reference) (OtherBodyIndex :type Integer))
  (bind _dialogui (Variables|Default|GetDialogUI))
  (Utilities|Casting|CastToBP_Character OtherActor)
  (Development|SetHiddeninGame (Variables|Default|GetInterraction_text) true false)
  (Utilities|IsValid _dialogui
    (:Is%20Valid
      (Widget|RemovefromParent _dialogui))))

(event Custom|reset%20Dialog
  (bind _dialogui (Variables|Default|GetDialogUI))
  (Utilities|FlowControl|DoOnce false) ; enters at Reset
)

(event EventBeginPlay)

(event Collision|EventActorBeginOverlap
  (params (OtherActor :type Actor%20Object%20Reference)))

(event EventTick
  (params (DeltaSeconds :type Float%20%28single-precision%29)))

(event EventEventDialogHappens
  (bind _dialogui (Variables|Default|GetDialogUI))
  (Utilities|FlowControl|DoOnce false
    (:Completed
      (Variables|/Game/BLUEPRINT/Dialog_system/Dialog_UI.Dialog_UI_C|Settext _dialogui (Variables|Default|GetNPC_txt))
      (Widget|SetVisibility (Variables|/Game/BLUEPRINT/Dialog_system/Dialog_UI.Dialog_UI_C|GetCanvasPanel_26 _dialogui) "Visible")
      (if (> (+ (Variables|/Game/BLUEPRINT/Dialog_system/Dialog_UI.Dialog_UI_C|Gettext-Index (Variables|Default|GetDialogUI)) 1) (- (Utilities|Array|Length (Variables|Default|GetNPC_txt)) 1))
        (Widget|RemovefromParent (Variables|Default|GetDialogUI))
        (CallFunction|ResetDialog)
        (else
          (Variables|/Game/BLUEPRINT/Dialog_system/Dialog_UI.Dialog_UI_C|Settext-Index (Variables|Default|GetDialogUI) (+ (Variables|/Game/BLUEPRINT/Dialog_system/Dialog_UI.Dialog_UI_C|Gettext-Index (Variables|Default|GetDialogUI)) 1))
          (CallFunction|ResetDialog))))))

(fn ConstructionScript)