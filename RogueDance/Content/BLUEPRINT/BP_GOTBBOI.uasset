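; BP_GOTBBOI is a 2D flipbook character whose animation follows the music bar by bar.
; On Tick it repeatedly subscribes to bar quantization events from a Quartz clock held by a Clock reference.
; The bar handler switches flipbooks at set bar counts, from idle through rap to power-up transitions.
; Along the way it moves the actor to the PosMid location cached at BeginPlay, then activates a particle system at the final stage.
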(event Custom|CustomEvent
  (params (ClockName :type Name) (QuantizationType :type EQuartzCommandQuantization%20Enum :default "Bar") (NumBars :type Integer) (Beat :type Integer) (BeatFraction :type Float%20%28single-precision%29))
  (bind _paperflipbook (Variables|Default|GetPaperFlipbook))
  (if (== NumBars 1)
    (Sprite|SetFlipbook (Variables|Default|GetPaperFlipbook) "/Game/ART/Darius/GOTBboy/Idle/GOTIdle.GOTIdle")
    (elif (== NumBars 10)
      (Sprite|SetFlipbook (Variables|Default|GetPaperFlipbook) "/Game/ART/Darius/GOTBboy/IdleRAP/_GOTidleRAP._GOTidleRAP")
      (elif (== 18 NumBars)
        (Sprite|SetFlipbook (Variables|Default|GetPaperFlipbook) "/Game/ART/Darius/GOTBboy/Powermove/GOTpowerloop.GOTpowerloop")
        (Transformation|SetActorLocation (Variables|Default|GetPosmidloc) false false)
        (elif (== NumBars 22)
          (Sprite|SetFlipbook (Variables|Default|GetPaperFlipbook) "/Game/ART/Darius/GOTBboy/Powermove/GOTpowerltrans.GOTpowerltrans")
          (elif (== NumBars 24)
            (Components|Timeline|SetLooping _paperflipbook true)
            (Sprite|SetFlipbook _paperflipbook "/Game/ART/Darius/GOTBboy/Powermove/GOTpowerltransFin.GOTpowerltransFin")
            (elif (== NumBars 26)
              (Sprite|SetFlipbook _paperflipbook "/Game/ART/Darius/GOTBboy/Powermove/GOTpowerltransFin1last.GOTpowerltransFin1last")
              (Components|Activation|Activate (Variables|Default|GetParticleSystem) false))))))))

(event EventBeginPlay
  (Variables|Default|SetPosmidloc (Transformation|GetActorLocation (Variables|Default|GetPosMid))))

(event Collision|EventActorBeginOverlap
  (params (OtherActor :type Actor%20Object%20Reference)))

(event EventTick
  (params (DeltaSeconds :type Float%20%28single-precision%29))
  (Class|QuartzClockHandle|SubscribetoQuantizationEvent (Variables|/Game/BLUEPRINT/DataAsset/DataAssetsAudio/BPD_Clock157.BPD_Clock157_C|GetClockTest (Variables|Default|GetClock)) "Bar" (delegate Custom|CustomEvent)))

(fn ConstructionScript)