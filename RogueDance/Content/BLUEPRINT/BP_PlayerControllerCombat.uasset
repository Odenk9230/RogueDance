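; BP_PlayerControllerCombat is the combat player controller, switching possession between the DPS, Tank and DJ crew characters.
; BeginPlay adds the input context, initializes crew health and stamina, and caches DPS and Tank, but sets DJ to None.
; Holding a select input possesses DJ or a phase-dependent dancer; release returns to DPS in attack phase, otherwise Tank.
; Tick reapplies BP_LevelCamCombat as view target, keeping the camera independent of possession.
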(event Input|EnhancedActionEvents|EnhancedInputActionIA_SelectDJ
  (params (ActionValue :type Boolean) (ElapsedSeconds :type Float%20%28double-precision%29) (TriggeredSeconds :type Float%20%28double-precision%29) (InputAction :type Input%20Action%20Object%20Reference :default "/Game/INPUT/InputActions/IA_SelectDJ.IA_SelectDJ"))
  (:Triggered
    (Pawn|Possess (Game|GetPlayerController 0) (Variables|Default|GetDJ)))
  (:Completed
    (Pawn|Possess (Game|GetPlayerController 0) (select (Variables|/Game/BLUEPRINT/DataAsset/DataAssetsGameplayElements/BPD_BattlePhase.BPD_BattlePhase_C|GetAttackPhase (Variables|Default|GetBattlePhase)) (Variables|Default|GetDPS) (Variables|Default|GetTank)))))

(event Input|EnhancedActionEvents|EnhancedInputActionIA_SelectDanseur2
  (params (ActionValue :type Boolean) (ElapsedSeconds :type Float%20%28double-precision%29) (TriggeredSeconds :type Float%20%28double-precision%29) (InputAction :type Input%20Action%20Object%20Reference :default "/Game/INPUT/InputActions/IA_SelectDanseur2.IA_SelectDanseur2"))
  (:Ongoing
    (Pawn|Possess (Game|GetPlayerController 0) (select (Variables|/Game/BLUEPRINT/DataAsset/DataAssetsGameplayElements/BPD_BattlePhase.BPD_BattlePhase_C|GetDefensePhase (Variables|Default|GetBattlePhase)) (Variables|Default|GetDPS) (Variables|Default|GetTank))))
  (:Completed
    (Pawn|Possess (Game|GetPlayerController 0) (select (Variables|/Game/BLUEPRINT/DataAsset/DataAssetsGameplayElements/BPD_BattlePhase.BPD_BattlePhase_C|GetAttackPhase (Variables|Default|GetBattlePhase)) (Variables|Default|GetDPS) (Variables|Default|GetTank)))))

(event EventBeginPlay
  (bind _staminabars (Variables|Default|GetStaminaBars))
  (Utilities|FlowControl|Sequence
    (:then_0
      ;[0.15 0.15 0.15 0.5] INIT INPUT
      (Input|AddMappingContext (PlayerController|LocalPlayerSubsystems|GetEnhancedInputLocalPlayerSubsystem self) "/Game/INPUT/MC_PlayerInputAlexCombat.MC_PlayerInputAlexCombat" 0 "(bIgnoreAllPressedKeysUntilRelease=True,bForceImmediately=False,bNotifyUserSettings=False)")
      ;[0.15 0.15 0.15 0.5] Set Up Health
      (Variables|/Game/BLUEPRINT/DataAsset/DataAssetRessources/BP_Health.BP_Health_C|SetHealthValue (Variables|Default|GetHealthCrew) 5e+01)
      ;[0.15 0.15 0.15 0.5] Set Up Stamina
      (Utilities|FlowControl|Sequence
        (:then_0
          (Variables|/Game/BLUEPRINT/DataAsset/DataAssetRessources/BPD_StaminaBar.BPD_StaminaBar_C|SetStaminaValueDps _staminabars (Variables|/Game/BLUEPRINT/DataAsset/DataAssetRessources/BPD_StaminaBar.BPD_StaminaBar_C|GetMaxStaminaValueDps _staminabars)))
        (:then_1
          (Variables|/Game/BLUEPRINT/DataAsset/DataAssetRessources/BPD_StaminaBar.BPD_StaminaBar_C|SetStaminaValueTank _staminabars (Variables|/Game/BLUEPRINT/DataAsset/DataAssetRessources/BPD_StaminaBar.BPD_StaminaBar_C|GetMaxStaminaValueTank _staminabars)))
        (:then_2
          (Variables|/Game/BLUEPRINT/DataAsset/DataAssetRessources/BPD_StaminaBar.BPD_StaminaBar_C|SetStaminaValueDj _staminabars (Variables|/Game/BLUEPRINT/DataAsset/DataAssetRessources/BPD_StaminaBar.BPD_StaminaBar_C|GetMaxStaminaValueDj _staminabars)))))
    (:then_1
      ;[0.15 0.15 0.15 0.5] CAMERA STAY WHERE IT NEED TO BE
      (bind _returnvalue (Actor|GetActorOfClass "/Game/BLUEPRINT/BP_LevelCamCombat.BP_LevelCamCombat_C"))
      (Game|Player|SetViewTargetwithBlend _returnvalue 0.0 "VTBlend_Linear" 0.0 false))
    (:then_2
      (Variables|Default|SetEnum "NewEnumerator1")
      (bind _returnvalue_2 (Actor|GetActorOfClass "/Game/BLUEPRINT/BP_Character.BP_Character_C"))
      (bind _asbp_character (Utilities|Casting|CastToBP_Character _returnvalue_2))
      (Variables|Default|SetDPS _asbp_character))
    (:then_3
      (bind _returnvalue_3 (Actor|GetActorOfClass "/Game/BLUEPRINT/BP_CharacterTank.BP_CharacterTank_C"))
      (bind _asbp_character_tank (Utilities|Casting|CastToBP_CharacterTank _returnvalue_3))
      (Variables|Default|SetTank _asbp_character_tank))
    (:then_4
      (bind _returnvalue_4 (Actor|GetActorOfClass "/Game/BLUEPRINT/BP_CharacterDJ.BP_CharacterDJ_C"))
      (Utilities|Casting|CastToBP_CharacterDJ _returnvalue_4)
      (Variables|Default|SetDJ 0))))

(event EventTick
  (params (DeltaSeconds :type Float%20%28single-precision%29))
  ;[0.15 0.15 0.15 0.5] CAMERA STAY WHERE IT NEED TO BE
  (bind _returnvalue (Actor|GetActorOfClass "/Game/BLUEPRINT/BP_LevelCamCombat.BP_LevelCamCombat_C"))
  (Game|Player|SetViewTargetwithBlend _returnvalue 0.0 "VTBlend_Linear" 0.0 false))

(fn ConstructionScript)