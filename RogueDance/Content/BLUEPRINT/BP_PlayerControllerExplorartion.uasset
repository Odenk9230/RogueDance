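; Player controller for exploration that drives the level's BP_Character while viewing it through a BP_LevelCam.
; On BeginPlay it adds the exploration Enhanced Input mapping context, sets the view target to the level camera, initializes an enum state, then finds and possesses the character.
; Tick looks up the level camera and reapplies it as view target every frame, keeping the view off the possessed pawn.
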(event EventBeginPlay
  (Utilities|FlowControl|Sequence
    (:then_0
      ;[0.15 0.15 0.15 0.5] INIT INPUT
      (Input|AddMappingContext (PlayerController|LocalPlayerSubsystems|GetEnhancedInputLocalPlayerSubsystem self) "/Game/INPUT/MC_PlayerInputExploration.MC_PlayerInputExploration" 0 "(bIgnoreAllPressedKeysUntilRelease=True,bForceImmediately=False,bNotifyUserSettings=False)"))
    (:then_1
      ;[0.15 0.15 0.15 0.5] CAMERA STAY WHERE IT NEED TO BE
      (bind _returnvalue (Actor|GetActorOfClass "/Game/BLUEPRINT/BP_LevelCam.BP_LevelCam_C"))
      (Game|Player|SetViewTargetwithBlend _returnvalue 0.0 "VTBlend_Linear" 0.0 false))
    (:then_2
      (Variables|Default|SetEnum "NewEnumerator0"))
    (:then_3
      (bind _returnvalue_2 (Actor|GetActorOfClass "/Game/BLUEPRINT/BP_Character.BP_Character_C"))
      (bind _asbp_character (Utilities|Casting|CastToBP_Character _returnvalue_2))
      (Variables|Default|SetChara _asbp_character))
    (:then_4
      (Pawn|Possess (Variables|Default|GetChara)))))

(event EventTick
  (params (DeltaSeconds :type Float%20%28single-precision%29))
  ;[0.15 0.15 0.15 0.5] CAMERA STAY WHERE IT NEED TO BE
  (bind _returnvalue (Actor|GetActorOfClass "/Game/BLUEPRINT/BP_LevelCam.BP_LevelCam_C"))
  (Game|Player|SetViewTargetwithBlend _returnvalue 0.0 "VTBlend_Linear" 0.0 false))

(fn ConstructionScript)