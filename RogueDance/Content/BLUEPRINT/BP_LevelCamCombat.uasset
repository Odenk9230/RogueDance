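; BP_LevelCamCombat is a level camera actor, going by its name, that tracks the character sideways along the Y axis.
; BeginPlay caches the BP_Charactertestcamera instance found in the level.
; While ModeMobat is false, Tick moves the actor to the character's Y plus Offset, truncated to an integer and clamped to hardcoded level bounds.
; Equal clamp limits pin X and Z to fixed values, so only Y varies.
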(event EventBeginPlay
  (bind _returnvalue (Actor|GetActorOfClass "/Game/BLUEPRINT/BP_Charactertestcamera.BP_Charactertestcamera_C"))
  (bind _asbp_charactertestcamera (Utilities|Casting|CastToBP_Charactertestcamera _returnvalue))
  (Variables|Default|SetCharacter1 _asbp_charactertestcamera))

(event Collision|EventActorBeginOverlap
  (params (OtherActor :type Actor%20Object%20Reference)))

(event EventTick
  (params (DeltaSeconds :type Float%20%28single-precision%29))
  (bind _character1 (Variables|Default|GetCharacter1))
  (bind _offset (Variables|Default|GetOffset))
  (bind _returnvalue (Transformation|GetActorLocation _character1))
  (bind _returnvalue_2 (+ (Math|Vector|MakeVector 0.0 (.y _returnvalue) (.z _returnvalue)) _offset))
  (if (not (Variables|Default|GetModeMobat))
    (Transformation|SetActorLocation (Math|Vector|MakeVector (Math|Conversions|ToFloat(Integer) (Math|Integer|Clamp(Integer) (Math|Float|Truncate (.x (Transformation|GetActorLocation))) -13248 -13248)) (Math|Conversions|ToFloat(Integer) (Math|Integer|Clamp(Integer) (Math|Float|Truncate (.y _returnvalue_2)) -10447 -4151)) (Math|Conversions|ToFloat(Integer) (Math|Integer|Clamp(Integer) (Math|Float|Truncate (.z _returnvalue_2)) 703 703))) false false)))

(fn ConstructionScript)