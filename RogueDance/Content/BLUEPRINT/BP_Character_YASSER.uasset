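; Playable flipbook dancer character that moves, triggers dialog on overlapping actors and performs dance combos and a held power move.
; Ability inputs advance a step-counted combo with timed resets; movement and dance flags feed AnimeStateMachine, which picks each tick's flipbook while possessed.
; When unpossessed outside the attack phase, it idles at its start position.
; A Quartz beat listener toggles an input window used only for debug printing; stamina refills every tick.
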(event Custom|UpdateAnimation
  ;[0.15 0.15 0.15 0.5] Set FlipBook
  (bind _output_get (Variables|Default|SetIsMoving (> (Math|Vector|VectorLength (Transformation|GetVelocity)) 0.0)))
  (bind _outputflipbook (CallFunction|AnimeStateMachine (Variables|Default|GetIsDancing) false (Variables|Default|GetWannaTop1) (Variables|Default|GetWannaTop2) (Variables|Default|GetWannaTop3) (Variables|Default|GetPowerMove) _output_get))
  (Sprite|SetFlipbook (Variables|Default|GetPaperFlipbook) _outputflipbook))

(event Custom|Input%20Listener%20On%20The%20Beat
  (params (ClockName :type Name) (QuantizationType :type EQuartzCommandQuantization%20Enum :default "Bar") (NumBars :type Integer) (Beat :type Integer) (BeatFraction :type Float%20%28single-precision%29))
  (switch Utilities|FlowControl|Switch|SwitchonEQuartzCommandQuantization QuantizationType
    (:Beat
      (if (== Beat 4)
        (Variables|Default|SetInputCheckerStart true)
        (elif (== Beat 1)
          (Variables|Default|SetInputCheckerStart false))))))

(event Input|EnhancedActionEvents|EnhancedInputActionIA_Face_Bottom
  (params (ActionValue :type Boolean) (ElapsedSeconds :type Float%20%28double-precision%29) (TriggeredSeconds :type Float%20%28double-precision%29) (InputAction :type Input%20Action%20Object%20Reference :default "/Game/INPUT/InputActions/IA_Face_Bottom.IA_Face_Bottom"))
  (:Completed
    (bind _array_element (Utilities|Array|ForEachLoopwithBreak (Collision|GetOverlappingActors 0 :!class /Script/Engine.Actor) :!label _label)
      (:LoopBody
        (if (Utilities|DoesObjectImplementInterface _array_element "/Game/BLUEPRINT/Dialog_system/Dialog_Interface.Dialog_Interface_C")
          (Class|DialogInterface|EventDialogHappens(Message) _array_element)
          (goto _label Break))))))

(event Input|EnhancedActionEvents|EnhancedInputActionIA_Ability2
  (params (ActionValue :type Boolean) (ElapsedSeconds :type Float%20%28double-precision%29) (TriggeredSeconds :type Float%20%28double-precision%29) (InputAction :type Input%20Action%20Object%20Reference :default "/Game/INPUT/InputActions/IA_Ability2.IA_Ability2"))
  ;[0.15 0.15 0.15 0.5] Ability Trigger Old
)

(event Input|EnhancedActionEvents|EnhancedInputActionIA_Ability3
  (params (ActionValue :type Boolean) (ElapsedSeconds :type Float%20%28double-precision%29) (TriggeredSeconds :type Float%20%28double-precision%29) (InputAction :type Input%20Action%20Object%20Reference :default "/Game/INPUT/InputActions/IA_Ability3.IA_Ability3"))
  ;[0.15 0.15 0.15 0.5] Ability Trigger Old
)

(event Input|EnhancedActionEvents|EnhancedInputActionIA_MoveZS
  (params (ActionValue :type Float%20%28double-precision%29) (ElapsedSeconds :type Float%20%28double-precision%29) (TriggeredSeconds :type Float%20%28double-precision%29) (InputAction :type Input%20Action%20Object%20Reference :default "/Game/INPUT/InputActions/IA_MoveZS.IA_MoveZS"))
  ;[0.06707 0.09097 0.15 0.5] Update Movement
  (if (not (Variables|Default|GetIsDancing))
    (Pawn|Input|AddMovementInput "1.000000,0.000000,0.000000" ActionValue false)))

(event Input|EnhancedActionEvents|EnhancedInputActionIA_MoveQD
  (params (ActionValue :type Float%20%28double-precision%29) (ElapsedSeconds :type Float%20%28double-precision%29) (TriggeredSeconds :type Float%20%28double-precision%29) (InputAction :type Input%20Action%20Object%20Reference :default "/Game/INPUT/InputActions/IA_MoveQD.IA_MoveQD"))
  ;[0.06707 0.09097 0.15 0.5] Update Movement
  (if (not (Variables|Default|GetIsDancing))
    (if (> ActionValue 0.0)
      (Variables|Default|SetBisMovingRight true)
      (elif (< ActionValue 0.0)
        (Variables|Default|SetBisMovingRight false)))
    (Pawn|Input|AddMovementInput "0.000000,1.000000,0.000000" ActionValue false)))

(event Input|EnhancedActionEvents|EnhancedInputActionIA_Controls_YBAX
  (params (ActionValue :type Boolean) (ElapsedSeconds :type Float%20%28double-precision%29) (TriggeredSeconds :type Float%20%28double-precision%29) (InputAction :type Input%20Action%20Object%20Reference :default "/Game/INPUT/InputActions/IA_Controls_YBAX.IA_Controls_YBAX"))
  ;[0.15 0.15 0.15 0.5] Ability Trigger Old
)

(event Input|EnhancedActionEvents|EnhancedInputActionIA_Ability2
  (params (ActionValue :type Boolean) (ElapsedSeconds :type Float%20%28double-precision%29) (TriggeredSeconds :type Float%20%28double-precision%29) (InputAction :type Input%20Action%20Object%20Reference :default "/Game/INPUT/InputActions/IA_Ability2.IA_Ability2"))
  ;[0.15 0.15 0.15 0.5] Combo System top Cross
  (if (Math|Boolean|ANDBoolean (Variables|AnimationCombo|GetIsInCombo) (Variables|Default|GetWannaTop1) (== (Variables|AnimationCombo|GetComboStep) 1))
    (Variables|AnimationCombo|SetComboStep (+ (Variables|AnimationCombo|GetComboStep) 1))
    (elif (Math|Boolean|ANDBoolean (Variables|AnimationCombo|GetIsInCombo) (Variables|Default|GetWannaTop1) (== (Variables|AnimationCombo|GetComboStep) 4))
      (Variables|AnimationCombo|SetComboStep (+ (Variables|AnimationCombo|GetComboStep) 1)))))

(event Input|EnhancedActionEvents|EnhancedInputActionIA_Ability3
  (params (ActionValue :type Boolean) (ElapsedSeconds :type Float%20%28double-precision%29) (TriggeredSeconds :type Float%20%28double-precision%29) (InputAction :type Input%20Action%20Object%20Reference :default "/Game/INPUT/InputActions/IA_Ability3.IA_Ability3"))
  ;[0.15 0.15 0.15 0.5] Combo System top Cross
  (if (Math|Boolean|ANDBoolean (Variables|AnimationCombo|GetIsInCombo) (Variables|Default|GetWannaTop1) (== (Variables|AnimationCombo|GetComboStep) 2))
    (Variables|AnimationCombo|SetComboStep (+ (Variables|AnimationCombo|GetComboStep) 1))
    (Utilities|FlowControl|Delay 1.0)
    (CallFunction|ResetAniminCombo)
    (elif (and (Variables|AnimationCombo|GetIsInCombo) (== (Variables|AnimationCombo|GetComboStep) 3))
      (Variables|Default|SetIsDancing true)
      (Variables|Default|SetWannaTop1 true)
      (Variables|AnimationCombo|SetComboStep (+ (Variables|AnimationCombo|GetComboStep) 1)))))

(event Input|EnhancedActionEvents|EnhancedInputActionIA_Ability4
  (params (ActionValue :type Boolean) (ElapsedSeconds :type Float%20%28double-precision%29) (TriggeredSeconds :type Float%20%28double-precision%29) (InputAction :type Input%20Action%20Object%20Reference :default "/Game/INPUT/InputActions/IA_Ability4.IA_Ability4"))
  ;[0.15 0.15 0.15 0.5] Ability Trigger Old
  (:Triggered
    (Variables|Default|SetIsDancing true)
    (Variables|Default|SetPowerMove true))
  (:Completed
    (Variables|Default|SetIsDancing false)
    (Variables|Default|SetPowerMove false)))

(event Input|EnhancedActionEvents|EnhancedInputActionIA_Controls_YBAX
  (params (ActionValue :type Boolean) (ElapsedSeconds :type Float%20%28double-precision%29) (TriggeredSeconds :type Float%20%28double-precision%29) (InputAction :type Input%20Action%20Object%20Reference :default "/Game/INPUT/InputActions/IA_Controls_YBAX.IA_Controls_YBAX"))
  (bind _staminaref (Variables|Default|GetStaminaRef))
  ;[0.15 0.15 0.15 0.5] Combo System top Cross
  (if (not (Variables|AnimationCombo|GetIsInCombo))
    (Variables|Default|SetIsDancing true)
    (Variables|Default|SetWannaTop1 true)
    (Variables|AnimationCombo|SetIsInCombo true)
    (Variables|AnimationCombo|SetComboStep (+ (Variables|AnimationCombo|GetComboStep) 1))
    (Variables|/Game/BLUEPRINT/DataAsset/DataAssetRessources/BPD_StaminaBar.BPD_StaminaBar_C|SetStaminaValueDps _staminaref (- (Variables|/Game/BLUEPRINT/DataAsset/DataAssetRessources/BPD_StaminaBar.BPD_StaminaBar_C|GetStaminaValueDps _staminaref) (Variables|Default|GetStaminaCostTop)))
    (Default|UpdateStaminaBars (Variables|Default|GetStamina))
    (elif (Math|Boolean|ANDBoolean (Variables|AnimationCombo|GetIsInCombo) (Variables|Default|GetWannaTop1) (== (Variables|AnimationCombo|GetComboStep) 5))
      (Variables|AnimationCombo|SetComboStep (+ (Variables|AnimationCombo|GetComboStep) 1))
      (Utilities|FlowControl|Delay 1.0)
      (CallFunction|ResetAnim))))

(event EventBeginPlay
  (Utilities|FlowControl|Sequence
    (:then_0
      (Variables|Default|SetBisMovingRight true)
      (Variables|Position|SetStartPosition (Transformation|GetActorLocation)))
    (:then_1
      (Variables|Default|SetClock%20157 (Variables|/Game/BLUEPRINT/DataAsset/DataAssetsAudio/BPD_Clock157.BPD_Clock157_C|GetClockTest (Variables|Default|GetRefClock))))
    (:then_2
      (Components|Timeline|SetLooping (Variables|Default|GetPaperFlipbook) true))))

(event Collision|EventActorBeginOverlap
  (params (OtherActor :type Actor%20Object%20Reference)))

(event EventTick
  (params (DeltaSeconds :type Float%20%28single-precision%29))
  (bind _returnvalue (Pawn|GetController))
  (bind _returnvalue_2 (Pawn|GetController))
  (bind _staminaref (Variables|Default|GetStaminaRef))
  (Utilities|FlowControl|Sequence
    (:then_1
      (if (Variables|Default|GetIsPossesed)
        ;[0.08409 0.07655 0.15 0.5] Update Anime On Tick
        (CallFunction|UpdateAnimation)
        (Math|Float|CompareFloat (.Y (Math|Vector|BreakVector (Variables|/Script/Engine.MovementComponent|GetVelocity (Pawn|GetMovementComponent)))) 0.0
          (:>
            (Utilities|IsValid _returnvalue_2 :!label _label
              (:Is%20Valid
                (Pawn|SetControlRotation _returnvalue_2 (Math|Rotator|MakeRotator 0.0 0.0 9e+01)))))
          (:==
            (if (Variables|Default|GetBisMovingRight)
              (goto _label)
              (else
                (Utilities|IsValid _returnvalue :!label _label_2
                  (:Is%20Valid
                    (Pawn|SetControlRotation _returnvalue (Math|Rotator|MakeRotator 0.0 0.0 -9e+01)))))))
          (:<
            (goto _label_2)))
        (elif (not (Variables|/Game/BLUEPRINT/DataAsset/DataAssetsGameplayElements/BPD_BattlePhase.BPD_BattlePhase_C|GetAttackPhase (Variables|Default|GetPhase)))
          (Sprite|SetFlipbook (Variables|Default|GetPaperFlipbook) (Variables|Animation|GetIdleFlipBook))
          (Transformation|SetActorLocation (Variables|Position|GetStartPosition) false false))))
    (:then_2
      (Utilities|FlowControl|DelayUntilNextTick)
      (Class|QuartzClockHandle|SubscribetoAllQuantizationEvents (Variables|Default|GetClock%20157) (delegate Custom|Input%20Listener%20On%20The%20Beat)))
    (:then_3
      (Variables|/Game/BLUEPRINT/DataAsset/DataAssetRessources/BPD_StaminaBar.BPD_StaminaBar_C|SetStaminaValueDps _staminaref (Variables|/Game/BLUEPRINT/DataAsset/DataAssetRessources/BPD_StaminaBar.BPD_StaminaBar_C|GetMaxStaminaValueDps _staminaref)))
    (:then_4
      (if (Math|Boolean|ANDBoolean (Variables|Default|GetInputCheckerStart) (Variables|Default|GetInput%20X) (Variables|Default|GetComboInput))
        (Development|PrintString "fresh")))))

(event EventPossessed
  (params (NewController :type Controller%20Object%20Reference))
  ;[0.15 0.15 0.15 0.5] Set Posseses Status for Use in The BP
  (Variables|Default|SetIsPossesed true))

(event EventUnpossessed
  (params (OldController :type Controller%20Object%20Reference))
  ;[0.15 0.15 0.15 0.5] Set Posseses Status for Use in The BP
  (Variables|Default|SetIsPossesed false))

(fn ConstructionScript)

(fn AnimeStateMachine
  (params (IsDancing :type Boolean) (WannaColl :type Boolean) (WannaTop1 :type Boolean) (WannaTop2 :type Boolean) (WannaTop3 :type Boolean) (WannaPower :type Boolean) (IsMoving :type Boolean))
  (if WannaColl
    (Variables|Animation|SetAnimastionState "NewEnumerator7")
    (else
      (if WannaTop1
        (Variables|Animation|SetAnimastionState "NewEnumerator2")
        (elif WannaTop2
          (Variables|Animation|SetAnimastionState "NewEnumerator3")
          (elif WannaTop3
            (Variables|Animation|SetAnimastionState "NewEnumerator4")
            (elif WannaPower
              (Variables|Animation|SetAnimastionState "NewEnumerator6")
              (elif IsMoving
                (Variables|Animation|SetAnimastionState "NewEnumerator1")
                (else
                  (Variables|Animation|SetAnimastionState "NewEnumerator0")))))))
      (return (Utilities|Select :Index (Variables|Animation|GetAnimastionState) :NewEnumerator0 (Variables|Animation|GetIdleFlipBook) :NewEnumerator1 (Variables|Animation|GetWalkFlipBook) :NewEnumerator2 (Utilities|Select :Index (Variables|AnimationCombo|GetComboCrossEnum) :NewEnumerator0 0 :NewEnumerator1 (Variables|AnimationCombo|GetCross2FB) :NewEnumerator2 0 :NewEnumerator3 0) :NewEnumerator3 (Variables|Animation|GetTopDance2FlipBook) :NewEnumerator4 (Variables|Animation|GetTopDance3FlipBook) :NewEnumerator5 (Variables|Animation|GetPowerPrepFlipBook) :NewEnumerator6 (Variables|Animation|GetPowerMoveFlipBook) :NewEnumerator7 (Variables|Animation|GetCollFlipBook))))))

(fn ResetAnim
  (Variables|Default|SetWannaTop1 false)
  (Variables|AnimationCombo|SetIsInCombo false)
  (Variables|Default|SetIsDancing false)
  (Variables|AnimationCombo|SetComboStep 0))

(fn ResetAniminCombo
  (Variables|Default|SetWannaTop1 false)
  (Variables|Default|SetIsDancing false)
  (Variables|AnimationCombo|SetComboStep 3))