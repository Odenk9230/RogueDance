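; Playable Paper2D/PaperZD character for rhythm-based dance combat, with movement and dialogue through Dialog_Interface on overlapping actors.
; Possession and combat phase toggle support status, which blocks movement.
; Ability inputs advance Cross, Spin and Down combo chains through step counters and flags.
; In Combat, Quartz beats open an input window where an animation flag triggers OnInputGood, counting hits and spawning slash VFX; the flipbook selector is unwired.
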(event Custom|UpdateAnimation
  ;[0.15 0.15 0.15 0.5] Set FlipBook
  (bind _output_get (Variables|Animation|SetIsMoving (> (Math|Vector|VectorLength (Transformation|GetVelocity)) 0.0))))

(event Custom|Input%20Listener%20On%20The%20Beat
  (params (ClockName :type Name) (QuantizationType :type EQuartzCommandQuantization%20Enum :default "Bar") (NumBars :type Integer) (Beat :type Integer) (BeatFraction :type Float%20%28single-precision%29))
  ;[0.15 0.15 0.15 0.5] INPUT LISTENER
  (switch Utilities|FlowControl|Switch|SwitchonEQuartzCommandQuantization QuantizationType
    (:Beat
      (if (== Beat 4)
        (Variables|InputChecker|SetInputCheckerStart true)
        (elif (== Beat 1)
          (Variables|InputChecker|SetInputCheckerStart false))))))

(event Custom|SpawnParticles
  (bind _returnvalue (Transformation|GetActorTransform))
  (bind (_roll _pitch _yaw) (Math|Rotator|BreakRotator (.rotation _returnvalue)))
  ;[0.15 0.15 0.15 0.5] Particles system
  (Niagara|SpawnSystematLocation (Variables|VFX|GetVFX%20Slash) (.location _returnvalue) (Math|Rotator|MakeRotator _roll _pitch (+ _yaw 9e+01)) (* (.scale _returnvalue) 2.0)))

(event Custom|UpdateProgressBar)

(event Custom|Update%20Stamina
  ;[0.15 0.15 0.15 0.5] INIT
  (|ReactToGoodInput))

(event Input|EnhancedActionEvents|EnhancedInputActionIA_Face_Bottom
  (params (ActionValue :type Boolean) (ElapsedSeconds :type Float%20%28double-precision%29) (TriggeredSeconds :type Float%20%28double-precision%29) (InputAction :type Input%20Action%20Object%20Reference :default "/Game/INPUT/InputActions/IA_Face_Bottom.IA_Face_Bottom"))
  (:Completed
    (bind _array_element (Utilities|Array|ForEachLoopwithBreak (Collision|GetOverlappingActors 0 :!class /Script/Engine.Actor) :!label _label)
      (:LoopBody
        (if (Utilities|DoesObjectImplementInterface _array_element "/Game/BLUEPRINT/Dialog_system/Dialog_Interface.Dialog_Interface_C")
          (Class|DialogInterface|EventDialogHappens(Message) _array_element)
          (goto _label Break))))))

(event Input|EnhancedActionEvents|EnhancedInputActionIA_Ability2
  (params (ActionValue :type Boolean) (ElapsedSeconds :type Float%20%28double-precision%29) (TriggeredSeconds :type Float%20%28double-precision%29) (InputAction :type Input%20Action%20Object%20Reference :default "/Game/INPUT/InputActions/IA_Ability2.IA_Ability2"))
  ;[0.15 0.15 0.15 0.5] Ability Trigger Old
)

(event Input|EnhancedActionEvents|EnhancedInputActionIA_Controls_YBAX
  (params (ActionValue :type Boolean) (ElapsedSeconds :type Float%20%28double-precision%29) (TriggeredSeconds :type Float%20%28double-precision%29) (InputAction :type Input%20Action%20Object%20Reference :default "/Game/INPUT/InputActions/IA_Controls_YBAX.IA_Controls_YBAX"))
  ;[0.15 0.15 0.15 0.5] Combo System top Cross
  (if (not (Variables|AnimationCombo|GetIsInCombo))
    (|Cross1 (Variables|AnimationCombo|GetComboStep))
    (elif (|ConditionStep4)
      (|Cross4 (Variables|AnimationCombo|GetComboStep))
      (|ResetAnimWithDelay)
      (|UpdateProgressBar))))

(event Input|EnhancedActionEvents|EnhancedInputActionIA_Ability2
  (params (ActionValue :type Boolean) (ElapsedSeconds :type Float%20%28double-precision%29) (TriggeredSeconds :type Float%20%28double-precision%29) (InputAction :type Input%20Action%20Object%20Reference :default "/Game/INPUT/InputActions/IA_Ability2.IA_Ability2"))
  ;[0.15 0.15 0.15 0.5] Combo System top Cross
  (if (|ConditionStep2)
    (|Cross2 (Variables|AnimationCombo|GetComboStep))))

(event Input|EnhancedActionEvents|EnhancedInputActionIA_Ability2
  (params (ActionValue :type Boolean) (ElapsedSeconds :type Float%20%28double-precision%29) (TriggeredSeconds :type Float%20%28double-precision%29) (InputAction :type Input%20Action%20Object%20Reference :default "/Game/INPUT/InputActions/IA_Ability2.IA_Ability2"))
  ;[0.15 0.15 0.15 0.5] Combo System top Spin
  (if (|ConditionSpinStep3)
    (|Spin2 (Variables|AnimationCombo|GetComboStep))))

(event Input|EnhancedActionEvents|EnhancedInputActionIA_Ability3
  (params (ActionValue :type Boolean) (ElapsedSeconds :type Float%20%28double-precision%29) (TriggeredSeconds :type Float%20%28double-precision%29) (InputAction :type Input%20Action%20Object%20Reference :default "/Game/INPUT/InputActions/IA_Ability3.IA_Ability3"))
  ;[0.15 0.15 0.15 0.5] Combo System top Spin
  (if (|ConditionSpinStep2_2)
    (|Spin1 (Variables|AnimationCombo|GetComboStep))))

(event Input|EnhancedActionEvents|EnhancedInputActionIA_Controls_YBAX
  (params (ActionValue :type Boolean) (ElapsedSeconds :type Float%20%28double-precision%29) (TriggeredSeconds :type Float%20%28double-precision%29) (InputAction :type Input%20Action%20Object%20Reference :default "/Game/INPUT/InputActions/IA_Controls_YBAX.IA_Controls_YBAX"))
  ;[0.15 0.15 0.15 0.5] Combo System top Spin
  (if (|ConditionSpinStep4)
    (|Spin3 (Variables|AnimationCombo|GetComboStep))
    (|ResetAnimWithDelay_2)))

(event Input|EnhancedActionEvents|EnhancedInputActionIA_Controls_YBAX
  (params (ActionValue :type Boolean) (ElapsedSeconds :type Float%20%28double-precision%29) (TriggeredSeconds :type Float%20%28double-precision%29) (InputAction :type Input%20Action%20Object%20Reference :default "/Game/INPUT/InputActions/IA_Controls_YBAX.IA_Controls_YBAX"))
  ;[0.15 0.15 0.15 0.5] Ability Trigger Old
  (|UpdateProgressBar_2))

(event Input|EnhancedActionEvents|EnhancedInputActionIA_Ability3
  (params (ActionValue :type Boolean) (ElapsedSeconds :type Float%20%28double-precision%29) (TriggeredSeconds :type Float%20%28double-precision%29) (InputAction :type Input%20Action%20Object%20Reference :default "/Game/INPUT/InputActions/IA_Ability3.IA_Ability3"))
  ;[0.15 0.15 0.15 0.5] Ability Trigger Old
)

(event Input|EnhancedActionEvents|EnhancedInputActionIA_MoveZS
  (params (ActionValue :type Float%20%28double-precision%29) (ElapsedSeconds :type Float%20%28double-precision%29) (TriggeredSeconds :type Float%20%28double-precision%29) (InputAction :type Input%20Action%20Object%20Reference :default "/Game/INPUT/InputActions/IA_MoveZS.IA_MoveZS"))
  ;[0.06707 0.09097 0.15 0.5] Update Movement
  (if (not (or (Variables|Default|GetIsSupport) (Variables|Animation|GetIsDancing)))
    (Pawn|Input|AddMovementInput "1.000000,0.000000,0.000000" ActionValue false)))

(event Input|EnhancedActionEvents|EnhancedInputActionIA_MoveQD
  (params (ActionValue :type Float%20%28double-precision%29) (ElapsedSeconds :type Float%20%28double-precision%29) (TriggeredSeconds :type Float%20%28double-precision%29) (InputAction :type Input%20Action%20Object%20Reference :default "/Game/INPUT/InputActions/IA_MoveQD.IA_MoveQD"))
  ;[0.06707 0.09097 0.15 0.5] Update Movement
  (if (not (or (Variables|Default|GetIsSupport) (Variables|Animation|GetIsDancing)))
    (if (> ActionValue 0.0)
      (Variables|Animation|SetBisMovingRight true)
      (elif (< ActionValue 0.0)
        (Variables|Animation|SetBisMovingRight false)))
    (Pawn|Input|AddMovementInput "0.000000,1.000000,0.000000" ActionValue false)))

(event Input|EnhancedActionEvents|EnhancedInputActionIA_Ability3
  (params (ActionValue :type Boolean) (ElapsedSeconds :type Float%20%28double-precision%29) (TriggeredSeconds :type Float%20%28double-precision%29) (InputAction :type Input%20Action%20Object%20Reference :default "/Game/INPUT/InputActions/IA_Ability3.IA_Ability3"))
  ;[0.15 0.15 0.15 0.5] Combo System top Cross
  (if (|ConditionStep3)
    (|Cross3 (Variables|AnimationCombo|GetComboStep))))

(event Input|EnhancedActionEvents|EnhancedInputActionIA_Ability2
  (params (ActionValue :type Boolean) (ElapsedSeconds :type Float%20%28double-precision%29) (TriggeredSeconds :type Float%20%28double-precision%29) (InputAction :type Input%20Action%20Object%20Reference :default "/Game/INPUT/InputActions/IA_Ability2.IA_Ability2"))
  ;[0.15 0.15 0.15 0.5] Combo System Down
  (if (not (and (Variables|AnimationCombo|GetIsInCombo) (Variables|Animation|GetWannaTop)))
    (|Down1 (Variables|AnimationCombo|GetComboStep))))

(event Input|EnhancedActionEvents|EnhancedInputActionIA_Ability3
  (params (ActionValue :type Boolean) (ElapsedSeconds :type Float%20%28double-precision%29) (TriggeredSeconds :type Float%20%28double-precision%29) (InputAction :type Input%20Action%20Object%20Reference :default "/Game/INPUT/InputActions/IA_Ability3.IA_Ability3"))
  ;[0.15 0.15 0.15 0.5] Combo System Down
  (if (|ConditionStep2Down)
    (|Down2 (Variables|AnimationCombo|GetComboStep))))

(event Input|EnhancedActionEvents|EnhancedInputActionIA_Ability4
  (params (ActionValue :type Boolean) (ElapsedSeconds :type Float%20%28double-precision%29) (TriggeredSeconds :type Float%20%28double-precision%29) (InputAction :type Input%20Action%20Object%20Reference :default "/Game/INPUT/InputActions/IA_Ability4.IA_Ability4"))
  ;[0.15 0.15 0.15 0.5] Ability Trigger Old
  (:Triggered
    (Variables|Animation|SetIsDancing true)
    (Variables|Animation|SetPowerMove true))
  (:Completed
    (Variables|Animation|SetIsDancing false)
    (Variables|Animation|SetPowerMove false)))

(event Input|EnhancedActionEvents|EnhancedInputActionIA_Controls_YBAX
  (params (ActionValue :type Boolean) (ElapsedSeconds :type Float%20%28double-precision%29) (TriggeredSeconds :type Float%20%28double-precision%29) (InputAction :type Input%20Action%20Object%20Reference :default "/Game/INPUT/InputActions/IA_Controls_YBAX.IA_Controls_YBAX"))
  ;[0.15 0.15 0.15 0.5] Combo System Down
  (if (|ConditionStep3down)
    (|SpinDown3 (Variables|AnimationCombo|GetComboStep))))

(event EventBeginPlay
  ;[0.15 0.15 0.15 0.5] INIT
  (Utilities|FlowControl|Sequence
    (:then_0
      (Variables|Animation|SetBisMovingRight true)
      (Variables|Position|SetStartPosition (Transformation|GetActorLocation)))
    (:then_1
      (EventDispatchers|BindEventtoOnInputGood (delegate Custom|Update%20Stamina)))
    (:then_2
      (Components|Timeline|SetLooping (Variables|Default|GetPaperFlipbook) true))))

(event EventTick
  (params (DeltaSeconds :type Float%20%28single-precision%29))
  (bind _returnvalue (Pawn|GetController))
  (bind _returnvalue_2 (Pawn|GetController))
  (Utilities|FlowControl|Sequence
    (:then_1
      ;[0.08409 0.07655 0.15 0.5] Update Anime On Tick
      (if (Variables|Animation|GetIsPossesed)
        (CallFunction|UpdateAnimation)
        (Math|Float|CompareFloat (.Y (Math|Vector|BreakVector (Variables|/Script/Engine.MovementComponent|GetVelocity (Pawn|GetMovementComponent)))) 0.0
          (:>
            (Utilities|IsValid _returnvalue_2 :!label _label
              (:Is%20Valid
                (Pawn|SetControlRotation _returnvalue_2 (Math|Rotator|MakeRotator 0.0 0.0 9e+01)))))
          (:==
            (if (Variables|Animation|GetBisMovingRight)
              (goto _label)
              (else
                (Utilities|IsValid _returnvalue :!label _label_2
                  (:Is%20Valid
                    (Pawn|SetControlRotation _returnvalue (Math|Rotator|MakeRotator 0.0 0.0 -9e+01)))))))
          (:<
            (goto _label_2)))
        (elif (not (Variables|/Game/BLUEPRINT/DataAsset/DataAssetsGameplayElements/BPD_BattlePhase.BPD_BattlePhase_C|GetAttackPhase (Variables|Phase|GetPhase)))
          (Sprite|SetFlipbook (Variables|Default|GetPaperFlipbook) (Variables|Animation|GetIdleFlipBook))
          (Transformation|SetActorLocation (Variables|Position|GetStartPosition) false false))))
    (:then_2
      (switch Utilities|FlowControl|Switch|SwitchonE_GameMode (Variables|Default|GetGameMode)
        (:NewEnumerator1
          ;[0.15 0.15 0.15 0.5] INPUT LISTENER
          (Class|QuartzClockHandle|SubscribetoAllQuantizationEvents (Variables|/Game/BLUEPRINT/DataAsset/DataAssetsAudio/BPD_Clock157.BPD_Clock157_C|GetClockTest (Variables|Quartz|GetRefClock)) (delegate Custom|Input%20Listener%20On%20The%20Beat)))))
    (:then_3
      (|StaminaValueSettings))
    (:then_4
      (|RefAnimator))
    (:then_5
      (if (Variables|InputChecker|GetInputCheckerStart)
        (if (Variables|InputChecker|GetInputListenerFromAnim)
          (Variables|InputChecker|SetInputListenerFromAnim false)
          (Variables|InputChecker|SetInputCheckerStart false)
          (Default|CallOnInputGood))
        (else
          (Variables|InputChecker|SetInputListenerFromAnim false))))))

(event EventPossessed
  (params (NewController :type Controller%20Object%20Reference))
  ;[0.15 0.15 0.15 0.5] Set Posseses Status for Use in The BP
  (Variables|Animation|SetIsPossesed true)
  (if (Variables|/Game/BLUEPRINT/DataAsset/DataAssetsGameplayElements/BPD_BattlePhase.BPD_BattlePhase_C|GetAttackPhase (Variables|Phase|GetPhase))
    (Variables|Default|SetIsSupport false)))

(event EventUnpossessed
  (params (OldController :type Controller%20Object%20Reference))
  ;[0.15 0.15 0.15 0.5] Set Posseses Status for Use in The BP
  (Variables|Animation|SetIsPossesed false)
  (if (Variables|/Game/BLUEPRINT/DataAsset/DataAssetsGameplayElements/BPD_BattlePhase.BPD_BattlePhase_C|GetDefensePhase (Variables|Phase|GetPhase))
    (Variables|Default|SetIsSupport true)
    (CallFunction|ResetAnim)))

(fn ConstructionScript)

(fn AnimeStateMachine
  (params (IsDancing :type Boolean) (WannaColl :type Boolean) (WannaTop1 :type Boolean) (WannaTop2 :type Boolean) (WannaTop3 :type Boolean) (WannaPower :type Boolean) (IsMoving :type Boolean))
  (if WannaColl
    (Variables|Animation|SetAnimastionState "NewEnumerator7")
    (else
      (if WannaTop1
        (Variables|Animation|SetAnimastionState "NewEnumerator2")
        (elif WannaTop2
          (Variables|Animation|SetAnimastionState "NewEnumerator3")
          (elif WannaTop3
            (Variables|Animation|SetAnimastionState "NewEnumerator4")
            (elif WannaPower
              (Variables|Animation|SetAnimastionState "NewEnumerator6")
              (elif IsMoving
                (Variables|Animation|SetAnimastionState "NewEnumerator1")
                (else
                  (Variables|Animation|SetAnimastionState "NewEnumerator0")))))))
      (return (Utilities|Select :Index (Variables|Animation|GetAnimastionState) :NewEnumerator0 (Variables|Animation|GetIdleFlipBook) :NewEnumerator1 (Variables|Animation|GetWalkFlipBook) :NewEnumerator2 (Utilities|Select :Index (Variables|AnimationCombo|GetComboCrossEnum) :NewEnumerator0 0 :NewEnumerator1 (Variables|AnimationCombo|GetCross2FB) :NewEnumerator2 0 :NewEnumerator3 0) :NewEnumerator3 (Variables|Animation|GetTopDance2FlipBook) :NewEnumerator4 (Variables|Animation|GetTopDance3FlipBook) :NewEnumerator5 (Variables|Animation|GetPowerPrepFlipBook) :NewEnumerator6 (Variables|Animation|GetPowerMoveFlipBook) :NewEnumerator7 (Variables|Animation|GetCollFlipBook))))))

(fn ResetAnim
  (if (Variables|Animation|GetWannaTopCross)
    (Variables|Animation|SetWannaTopCross false)
    (Variables|AnimationCombo|SetIsInCombo false :!label _label)
    (Variables|Animation|SetWannaTop false)
    (Variables|Animation|SetWannaDown false)
    (Variables|Animation|SetIsDancing false)
    (Variables|AnimationCombo|SetComboStep 0)
    (Variables|Animation|SetIsMoving false)
    (elif (Variables|Animation|GetWannaTopSpin)
      (Variables|Animation|SetWannaTopSpin false)
      (goto _label)
      (elif (Variables|Animation|GetWannaDown)
        (Variables|Animation|SetWannaDown false)
        (goto _label)))))

(fn ResetAniminCombo
  (Variables|Animation|SetWannaTopCross false)
  (Variables|Animation|SetIsDancing false)
  (Variables|AnimationCombo|SetComboStep 3))