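; BP_2DCharacter is a flipbook-animated 2D character moved by Enhanced Input.
; Forward and right input actions add movement along fixed world X and Y axes.
; AnimStateMachine sets an Idle, Walk or Dance state and returns the matching flipbook.
; Its only call, which derives movement from velocity and fixes dancing to false, is disconnected, and UpdateAnimation is empty, so the graph never switches animations.
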(event Custom|UpdateAnimation)

(event Input|EnhancedActionEvents|EnhancedInputActionIA_MoveFwd
  (params (ActionValue :type Float%20%28double-precision%29) (ElapsedSeconds :type Float%20%28double-precision%29) (TriggeredSeconds :type Float%20%28double-precision%29) (InputAction :type Input%20Action%20Object%20Reference :default "/Game/INPUT/InputActions/IA_MoveFwd.IA_MoveFwd"))
  (Pawn|Input|AddMovementInput "1.000000,0.000000,0.000000" ActionValue false))

(event Input|EnhancedActionEvents|EnhancedInputActionIA_MoveRight
  (params (ActionValue :type Float%20%28double-precision%29) (ElapsedSeconds :type Float%20%28double-precision%29) (TriggeredSeconds :type Float%20%28double-precision%29) (InputAction :type Input%20Action%20Object%20Reference :default "/Game/INPUT/InputActions/IA_MoveRight.IA_MoveRight"))
  (Pawn|Input|AddMovementInput "0.000000,1.000000,0.000000" ActionValue false))

(event EventBeginPlay)

(event Collision|EventActorBeginOverlap
  (params (OtherActor :type Actor%20Object%20Reference)))

(event EventTick
  (params (DeltaSeconds :type Float%20%28single-precision%29)))

(fn ConstructionScript)

(fn AnimStateMachine
  (params (IsDancing :type Boolean) (IsMoving :type Boolean))
  (if IsDancing
    (Variables|Animation|SetAnimeState "NewEnumerator2")
    (elif IsMoving
      (Variables|Animation|SetAnimeState "NewEnumerator1")
      (else
        (Variables|Animation|SetAnimeState "NewEnumerator0"))))
  (return (Utilities|Select :Index (Variables|Animation|GetAnimeState) :NewEnumerator0 (Variables|Animation|GetIdleFlipBook) :NewEnumerator1 (Variables|Animation|GetWalkFlipBook) :NewEnumerator2 (Variables|Animation|GetDanceFlipBook))))