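; BP_LevelCam is a level camera actor that follows BP_Character sideways along the world Y axis.
; BeginPlay finds and caches the character reference.
; Each Tick sets the actor's location from the character's Y plus an offset, clamped to hardcoded level bounds.
; Identical min and max clamps lock X and Z to constants, and all coordinates are truncated to whole units.
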(event EventBeginPlay
  (bind _returnvalue (Actor|GetActorOfClass "/Game/BLUEPRINT/BP_Character.BP_Character_C"))
  (bind _asbp_character (Utilities|Casting|CastToBP_Character _returnvalue))
  (Variables|Default|SetCharacter1_0 _asbp_character))

(event Collision|EventActorBeginOverlap
  (params (OtherActor :type Actor%20Object%20Reference)))

(event EventTick
  (params (DeltaSeconds :type Float%20%28single-precision%29))
  (bind _character1_0 (Variables|Default|GetCharacter1_0))
  (bind _offset (Variables|Default|GetOffset))
  (bind _returnvalue (Transformation|GetActorLocation _character1_0))
  (bind _returnvalue_2 (+ (Math|Vector|MakeVector 0.0 (.y _returnvalue) (.z _returnvalue)) _offset))
  (Transformation|SetActorLocation (Math|Vector|MakeVector (Math|Conversions|ToFloat(Integer) (Math|Integer|Clamp(Integer) (Math|Float|Truncate (.x (Transformation|GetActorLocation))) -13248 -13248)) (Math|Conversions|ToFloat(Integer) (Math|Integer|Clamp(Integer) (Math|Float|Truncate (.y _returnvalue_2)) -10447 -4151)) (Math|Conversions|ToFloat(Integer) (Math|Integer|Clamp(Integer) (Math|Float|Truncate (.z _returnvalue_2)) 703 703))) false false))

(fn ConstructionScript)