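; Test player character or pawn, named for a follow-camera test, that moves from Enhanced Input actions.
; IA_MoveZS and IA_MoveQD add movement input along fixed world X and Y axes, so direction ignores camera and control rotation.
; Tick and BeginPlay are empty, and the graph holds no camera logic.
; Leftover self-possess and yaw-relative direction nodes are disconnected and never run.
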(event Input|EnhancedActionEvents|EnhancedInputActionIA_MoveZS
  (params (ActionValue :type Float%20%28double-precision%29) (ElapsedSeconds :type Float%20%28double-precision%29) (TriggeredSeconds :type Float%20%28double-precision%29) (InputAction :type Input%20Action%20Object%20Reference :default "/Game/INPUT/InputActions/IA_MoveZS.IA_MoveZS"))
  (Pawn|Input|AddMovementInput "1.000000,0.000000,0.000000" ActionValue false))

(event Input|EnhancedActionEvents|EnhancedInputActionIA_MoveQD
  (params (ActionValue :type Float%20%28double-precision%29) (ElapsedSeconds :type Float%20%28double-precision%29) (TriggeredSeconds :type Float%20%28double-precision%29) (InputAction :type Input%20Action%20Object%20Reference :default "/Game/INPUT/InputActions/IA_MoveQD.IA_MoveQD"))
  (Pawn|Input|AddMovementInput "0.000000,1.000000,0.000000" ActionValue false))

(event EventBeginPlay)

(event Collision|EventActorBeginOverlap
  (params (OtherActor :type Actor%20Object%20Reference)))

(event EventTick
  (params (DeltaSeconds :type Float%20%28single-precision%29)))

(fn ConstructionScript)