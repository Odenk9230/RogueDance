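; Level camera actor for exploration that follows the exploration character along a side-on plane.
; On BeginPlay it caches the BP_CharacterExploration found in the level.
; Each Tick, unless ModeMobat is set, it adds Offset to the character's Y and Z, clamps them to hard-coded bounds, pins X to a constant, then adds OffsetBoiteDeNuit before moving itself.
; A lookup of BP_Character is left unconnected.
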(event EventBeginPlay
  (bind _returnvalue (Actor|GetActorOfClass "/Game/BLUEPRINT/BP_CharacterExploration.BP_CharacterExploration_C"))
  (bind _asbp_character_exploration (Utilities|Casting|CastToBP_CharacterExploration _returnvalue))
  (Variables|Default|SetChara%20explo _asbp_character_exploration))

(event Collision|EventActorBeginOverlap
  (params (OtherActor :type Actor%20Object%20Reference)))

(event EventTick
  (params (DeltaSeconds :type Float%20%28single-precision%29))
  (bind _chara_explo (Variables|Default|GetChara%20explo))
  (bind _offset_boite_de_nuit (Variables|Default|GetOffset_boite%20de%20nuit))
  (bind _offset (Variables|Default|GetOffset))
  (bind _returnvalue (Transformation|GetActorLocation _chara_explo))
  (bind _returnvalue_2 (+ (Math|Vector|MakeVector 0.0 (.y _returnvalue) (.z _returnvalue)) _offset))
  (bind _returnvalue_3 (Math|Float|Truncate (.z _returnvalue_2)))
  (bind _returnvalue_4 (Math|Float|Truncate (.y _returnvalue_2)))
  (bind _returnvalue_5 (Math|Integer|Clamp(Integer) _returnvalue_3 663 2713))
  (bind _returnvalue_6 (Math|Integer|Clamp(Integer) _returnvalue_4 -9856 -4284))
  (bind _returnvalue_7 (Math|Conversions|ToFloat(Integer) _returnvalue_5))
  (bind _returnvalue_8 (Math|Conversions|ToFloat(Integer) _returnvalue_6))
  (bind _returnvalue_9 (Math|Vector|MakeVector 0.0 _returnvalue_8 _returnvalue_7))
  (bind _returnvalue_10 (+ _returnvalue_9 _offset_boite_de_nuit))
  (if (not (Variables|Default|GetModeMobat))
    (Transformation|SetActorLocation (Math|Vector|MakeVector (+ (Math|Conversions|ToFloat(Integer) (Math|Integer|Clamp(Integer) (Math|Float|Truncate (.x (Transformation|GetActorLocation))) -13248 -13248)) (.x _returnvalue_10)) (.y _returnvalue_10) (.z _returnvalue_10)) false false)))

(fn ConstructionScript)