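; Paper2D DJ character that moves on two axes and can buff while a button is held, which blocks movement input.
; Each Tick picks an Idle, Walk, Cheer or Buff flipbook through AnimeStateMachine, with Cheer first, then Buff, then Walk.
; Tick also snaps control yaw to one of two opposite facings from X velocity, falling back on the last left/right input when that is zero.
; IsCheering is only read here, never set.
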(event Custom|UpdateAnimation
  (bind _output_get (Variables|Default|SetIsMoving (> (Math|Vector|VectorLength (Transformation|GetVelocity)) 0.0)))
  (bind _outputflipbook (CallFunction|AnimeStateMachine _output_get (Variables|Default|GetIsCheering) (Variables|Default|GetIsBuffing)))
  (Sprite|SetFlipbook (Variables|Default|GetPaperFlipbook) _outputflipbook))

(event Input|EnhancedActionEvents|EnhancedInputActionIA_Controls_YBAX
  (params (ActionValue :type Boolean) (ElapsedSeconds :type Float%20%28double-precision%29) (TriggeredSeconds :type Float%20%28double-precision%29) (InputAction :type Input%20Action%20Object%20Reference :default "/Game/INPUT/InputActions/IA_Controls_YBAX.IA_Controls_YBAX"))
  (:Triggered
    (Variables|Default|SetIsBuffing true))
  (:Completed
    (Variables|Default|SetIsBuffing false)))

(event Input|EnhancedActionEvents|EnhancedInputActionIA_MoveZS
  (params (ActionValue :type Float%20%28double-precision%29) (ElapsedSeconds :type Float%20%28double-precision%29) (TriggeredSeconds :type Float%20%28double-precision%29) (InputAction :type Input%20Action%20Object%20Reference :default "/Game/INPUT/InputActions/IA_MoveZS.IA_MoveZS"))
  ;[0.06707 0.09097 0.15 0.5] Update Movement
  (if (not (Variables|Default|GetIsBuffing))
    (Pawn|Input|AddMovementInput "1.000000,0.000000,0.000000" ActionValue false)))

(event Input|EnhancedActionEvents|EnhancedInputActionIA_MoveQD
  (params (ActionValue :type Float%20%28double-precision%29) (ElapsedSeconds :type Float%20%28double-precision%29) (TriggeredSeconds :type Float%20%28double-precision%29) (InputAction :type Input%20Action%20Object%20Reference :default "/Game/INPUT/InputActions/IA_MoveQD.IA_MoveQD"))
  ;[0.06707 0.09097 0.15 0.5] Update Movement
  (if (not (Variables|Default|GetIsBuffing))
    (if (> ActionValue 0.0)
      (Variables|Default|SetBisMovingRight true)
      (elif (< ActionValue 0.0)
        (Variables|Default|SetBisMovingRight false)))
    (Pawn|Input|AddMovementInput "0.000000,1.000000,0.000000" ActionValue false)))

(event EventBeginPlay)

(event Collision|EventActorBeginOverlap
  (params (OtherActor :type Actor%20Object%20Reference)))

(event EventTick
  (params (DeltaSeconds :type Float%20%28single-precision%29))
  (bind _returnvalue (Pawn|GetController))
  (bind _returnvalue_2 (Pawn|GetController))
  (Utilities|FlowControl|Sequence
    (:then_1
      ;[0.08409 0.07655 0.15 0.5] Update Anime On Tick
      (CallFunction|UpdateAnimation)
      (Math|Float|CompareFloat (.X (Math|Vector|BreakVector (Variables|/Script/Engine.MovementComponent|GetVelocity (Pawn|GetMovementComponent)))) 0.0
        (:>
          (Utilities|IsValid _returnvalue_2 :!label _label
            (:Is%20Valid
              (Pawn|SetControlRotation _returnvalue_2 (Math|Rotator|MakeRotator 0.0 0.0 -9e+01)))))
        (:==
          (if (Variables|Default|GetBisMovingRight)
            (goto _label)
            (else
              (Utilities|IsValid _returnvalue :!label _label_2
                (:Is%20Valid
                  (Pawn|SetControlRotation _returnvalue (Math|Rotator|MakeRotator 0.0 0.0 9e+01)))))))
        (:<
          (goto _label_2))))))

(fn ConstructionScript)

(fn AnimeStateMachine
  (params (IsMoving :type Boolean) (IsCheering :type Boolean) (IsBuffing :type Boolean))
  (if IsCheering
    (Variables|Animation|SetAnimastionState "NewEnumerator3")
    (elif IsBuffing
      (Variables|Animation|SetAnimastionState "NewEnumerator4")
      (elif IsMoving
        (Variables|Animation|SetAnimastionState "NewEnumerator1")
        (else
          (Variables|Animation|SetAnimastionState "NewEnumerator0")))))
  (return (Utilities|Select :Index (Variables|Animation|GetAnimastionState) :NewEnumerator0 (Variables|Animation|GetIdleFlipBook) :NewEnumerator1 (Variables|Animation|GetWalkFlipBook) :NewEnumerator3 (Variables|Animation|GetCheerFlipBook) :NewEnumerator4 (Variables|Animation|GetBuffFlipBook))))