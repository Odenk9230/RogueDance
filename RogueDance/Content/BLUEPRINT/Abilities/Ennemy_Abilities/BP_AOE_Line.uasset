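; BP_AOE_Line is an enemy line AOE ability actor that telegraphs a location, then fires a projectile.
; BeginPlay copies positions from RefAoeLoc, clearing that list first if it holds four or more, and hides the AOELINE indicator.
; SpawnAOE moves to a random position, shows the indicator, waits briefly, then spawns BP_Projectile at an offset.
; An unconnected branch would instead gather positions from BP_AOELinePosition actors.
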(event Custom|DespaawnAOE
  (Rendering|SetVisibility (Variables|Default|GetAOE%20LINE) false false))

(event Custom|Spawn%20Projectile
  (Game|SpawnActorfromClass "/Game/BLUEPRINT/Abilities/Ennemy_Abilities/BP_Projectile.BP_Projectile_C" (Math|Conversions|ToTransform(Vector) (+ (Variables|Default|GetChosePos) (Variables|Default|GetOffset))) "Undefined" "MultiplyWithRoot" 0 0))

(event Custom|SpawnAOE
  (bind _output_get (Variables|Default|SetChosePos (.OutItem (Utilities|Array|Random (Variables|Default|GetPositions)))))
  (Transformation|SetActorLocation _output_get false false)
  (Rendering|SetVisibility (Variables|Default|GetAOE%20LINE) true false)
  (Utilities|FlowControl|Delay 1.0)
  (CallFunction|SpawnProjectile))

(event EventBeginPlay
  (bind _refaoeloc (Variables|Default|GetRefAoeLoc))
  (bind _lineaoelocation (Variables|/Game/BLUEPRINT/DataAsset/BPD_AOELOCATION.BPD_AOELOCATION_C|GetLineAoeLocation _refaoeloc))
  (if (>= (Utilities|Array|Length _lineaoelocation) 4)
    (Utilities|Array|Clear _lineaoelocation))
  (bind _output_get (Variables|Default|SetPositions _lineaoelocation))
  (Development|PrintString (Utilities|String|ToString(Integer) (Utilities|Array|Length _output_get)))
  (CallFunction|DespaawnAOE))

(event EventTick
  (params (DeltaSeconds :type Float%20%28single-precision%29)))

(fn ConstructionScript)