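; Enemy line area-of-effect ability actor, likely for the skatepark, that shows an AOE line indicator and fires a projectile.
; SpawnAOE moves it to a random stored position plus an offset and reveals the line, which is hidden on BeginPlay and by DespaawnAOE.
; SpawnProjectile spawns BP_Projectile at that offset position.
; Tick re-arms a short timer each frame to copy positions from RefAoeLoc; an actor-gathering alternative is unconnected.
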(event Custom|DespaawnAOE
  (Rendering|SetVisibility (Variables|Default|GetAOE%20LINE) false false))

(event Custom|Spawn%20Projectile
  (Game|SpawnActorfromClass "/Game/BLUEPRINT/Abilities/Ennemy_Abilities/BP_Projectile.BP_Projectile_C" (Math|Transform|MakeTransform (+ (Variables|Default|GetChosePos) (Variables|Default|GetOffset)) (Variables|Default|GetOffset%20Rotation%20Projectile) "1.000000,1.000000,1.000000") "Undefined" "MultiplyWithRoot" 0 0))

(event Custom|SpawnAOE
  (params (Offset :type Vector))
  (bind _output_get (Variables|Default|SetChosePos (.OutItem (Utilities|Array|Random (Variables|Default|GetPositions)))))
  (Transformation|SetActorLocation (+ _output_get Offset) false false)
  (Rendering|SetVisibility (Variables|Default|GetAOE%20LINE) true false))

(event Custom|Set%20Pos
  (Variables|Default|SetPositions (Variables|/Game/BLUEPRINT/DataAsset/DataAssetsGameplayElements/BPD_AOELOCATION.BPD_AOELOCATION_C|GetLineAoeLocation (Variables|Default|GetRefAoeLoc))))

(event EventBeginPlay
  (CallFunction|DespaawnAOE))

(event EventTick
  (params (DeltaSeconds :type Float%20%28single-precision%29))
  (Utilities|FlowControl|Sequence
    (:then_0
      (Utilities|Time|SetTimerbyEvent (delegate Custom|Set%20Pos) 0.2))))

(fn ConstructionScript)