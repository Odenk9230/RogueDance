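; Exploration character with flipbook animations that walks on two input axes, with movement blocked while supporting or dancing.
; Tick updates IsMoving and snaps controller yaw left or right from Y velocity, keeping the last input direction when Y velocity is zero.
; Dance-reset functions clear combo flags, and SpawnParticles emits a slash effect.
; AnimeStateMachine selects idle, walk, dance or power flipbooks, but its event-graph call never runs.
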(event Custom|UpdateAnimation
  (bind _output_get (Variables|Animation|SetIsMoving (> (Math|Vector|VectorLength (Transformation|GetVelocity)) 0.0))))

(event Custom|SpawnParticles
  (bind _returnvalue (Transformation|GetActorTransform))
  (bind (_roll _pitch _yaw) (Math|Rotator|BreakRotator (.rotation _returnvalue)))
  ;[0.15 0.15 0.15 0.5] Particles system
  (Niagara|SpawnSystematLocation (Variables|VFX|GetVFX%20Slash) (.location _returnvalue) (Math|Rotator|MakeRotator _roll _pitch (+ _yaw 9e+01)) (* (.scale _returnvalue) 2.0)))

(event Input|EnhancedActionEvents|EnhancedInputActionIA_MoveZS
  (params (ActionValue :type Float%20%28double-precision%29) (ElapsedSeconds :type Float%20%28double-precision%29) (TriggeredSeconds :type Float%20%28double-precision%29) (InputAction :type Input%20Action%20Object%20Reference :default "/Game/INPUT/InputActions/IA_MoveZS.IA_MoveZS"))
  ;[0.06707 0.09097 0.15 0.5] Update Movement
  (if (not (or (Variables|Default|GetIsSupport) (Variables|Animation|GetIsDancing)))
    (Pawn|Input|AddMovementInput "1.000000,0.000000,0.000000" ActionValue false)))

(event Input|EnhancedActionEvents|EnhancedInputActionIA_MoveQD
  (params (ActionValue :type Float%20%28double-precision%29) (ElapsedSeconds :type Float%20%28double-precision%29) (TriggeredSeconds :type Float%20%28double-precision%29) (InputAction :type Input%20Action%20Object%20Reference :default "/Game/INPUT/InputActions/IA_MoveQD.IA_MoveQD"))
  ;[0.06707 0.09097 0.15 0.5] Update Movement
  (if (not (or (Variables|Default|GetIsSupport) (Variables|Animation|GetIsDancing)))
    (if (> ActionValue 0.0)
      (Variables|Animation|SetBisMovingRight true)
      (elif (< ActionValue 0.0)
        (Variables|Animation|SetBisMovingRight false)))
    (Pawn|Input|AddMovementInput "0.000000,1.000000,0.000000" ActionValue false)))

(event EventBeginPlay
  ;[0.15 0.15 0.15 0.5] INIT
  (Utilities|FlowControl|Sequence
    (:then_0
      (Variables|Animation|SetBisMovingRight true))))

(event EventTick
  (params (DeltaSeconds :type Float%20%28single-precision%29))
  (bind _returnvalue (Pawn|GetController))
  (bind _returnvalue_2 (Pawn|GetController))
  (Utilities|FlowControl|Sequence
    (:then_1
      ;[0.08409 0.07655 0.15 0.5] Update Anime On Tick
      (if true
        (CallFunction|UpdateAnimation)
        (Math|Float|CompareFloat (.Y (Math|Vector|BreakVector (Variables|/Script/Engine.MovementComponent|GetVelocity (Pawn|GetMovementComponent)))) 0.0
          (:>
            (Utilities|IsValid _returnvalue_2 :!label _label
              (:Is%20Valid
                (Pawn|SetControlRotation _returnvalue_2 (Math|Rotator|MakeRotator 0.0 0.0 9e+01)))))
          (:==
            (if (Variables|Animation|GetBisMovingRight)
              (goto _label)
              (else
                (Utilities|IsValid _returnvalue :!label _label_2
                  (:Is%20Valid
                    (Pawn|SetControlRotation _returnvalue (Math|Rotator|MakeRotator 0.0 0.0 -9e+01)))))))
          (:<
            (goto _label_2)))))))

(fn ConstructionScript)

(fn AnimeStateMachine
  (params (IsDancing :type Boolean) (WannaColl :type Boolean) (WannaTop1 :type Boolean) (WannaTop2 :type Boolean) (WannaTop3 :type Boolean) (WannaPower :type Boolean) (IsMoving :type Boolean))
  (if WannaColl
    (Variables|Animation|SetAnimastionState "NewEnumerator7")
    (else
      (if WannaTop1
        (Variables|Animation|SetAnimastionState "NewEnumerator2")
        (elif WannaTop2
          (Variables|Animation|SetAnimastionState "NewEnumerator3")
          (elif WannaTop3
            (Variables|Animation|SetAnimastionState "NewEnumerator4")
            (elif WannaPower
              (Variables|Animation|SetAnimastionState "NewEnumerator6")
              (elif IsMoving
                (Variables|Animation|SetAnimastionState "NewEnumerator1")
                (else
                  (Variables|Animation|SetAnimastionState "NewEnumerator0")))))))
      (return (Utilities|Select :Index (Variables|Animation|GetAnimastionState) :NewEnumerator0 (Variables|Animation|GetIdleFlipBook) :NewEnumerator1 (Variables|Animation|GetWalkFlipBook) :NewEnumerator2 (Utilities|Select :Index (Variables|AnimationCombo|GetComboCrossEnum) :NewEnumerator0 0 :NewEnumerator1 (Variables|AnimationCombo|GetCross2FB) :NewEnumerator2 0 :NewEnumerator3 0) :NewEnumerator3 (Variables|Animation|GetTopDance2FlipBook) :NewEnumerator4 (Variables|Animation|GetTopDance3FlipBook) :NewEnumerator5 (Variables|Animation|GetPowerPrepFlipBook) :NewEnumerator6 (Variables|Animation|GetPowerMoveFlipBook) :NewEnumerator7 (Variables|Animation|GetCollFlipBook))))))

(fn ResetAnim
  (if (Variables|Animation|GetWannaTopCross)
    (Variables|Animation|SetWannaTopCross false)
    (Variables|AnimationCombo|SetIsInCombo false :!label _label)
    (Variables|Animation|SetWannaTop false)
    (Variables|Animation|SetWannaDown false)
    (Variables|Animation|SetIsDancing false)
    (Variables|AnimationCombo|SetComboStep 0)
    (Variables|Animation|SetIsMoving false)
    (elif (Variables|Animation|GetWannaTopSpin)
      (Variables|Animation|SetWannaTopSpin false)
      (goto _label)
      (elif (Variables|Animation|GetWannaDown)
        (Variables|Animation|SetWannaDown false)
        (goto _label)
        (elif (Variables|Animation|GetPowerMove)
          (Variables|Animation|SetPowerMove false)
          (goto _label))))))

(fn ResetAniminCombo
  (Variables|Animation|SetWannaTopCross false)
  (Variables|Animation|SetIsDancing false)
  (Variables|AnimationCombo|SetComboStep 3))