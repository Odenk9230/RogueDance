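; Exploration camera actor for the nightclub (boîte de nuit) level that positions itself from the player's BP_Character location.
; BeginPlay caches the character, and Tick moves the actor while ModeMobat is false.
; X is pinned to a constant, while Y and Z take the character's position plus Offset, are integer-clamped, then shifted by OffsetBoiteDeNuit.
; The Y clamp has its Min and Max reversed.
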(event EventBeginPlay
  (bind _returnvalue (Actor|GetActorOfClass "/Game/BLUEPRINT/BP_Character.BP_Character_C"))
  (bind _asbp_character (Utilities|Casting|CastToBP_Character _returnvalue))
  (Variables|Default|SetCharacter _asbp_character))

(event Collision|EventActorBeginOverlap
  (params (OtherActor :type Actor%20Object%20Reference)))

(event EventTick
  (params (DeltaSeconds :type Float%20%28single-precision%29))
  (bind _character (Variables|Default|GetCharacter))
  (bind _offset_boite_de_nuit (Variables|Default|GetOffset_boite%20de%20nuit))
  (bind _offset (Variables|Default|GetOffset))
  (bind _returnvalue (Transformation|GetActorLocation _character))
  (bind _returnvalue_2 (+ (Math|Vector|MakeVector 0.0 (.y _returnvalue) (.z _returnvalue)) _offset))
  (bind _returnvalue_3 (Math|Float|Truncate (.z _returnvalue_2)))
  (bind _returnvalue_4 (Math|Float|Truncate (.y _returnvalue_2)))
  (bind _returnvalue_5 (Math|Integer|Clamp(Integer) _returnvalue_3 995 2713))
  (bind _returnvalue_6 (Math|Integer|Clamp(Integer) _returnvalue_4 -4626 -10058))
  (bind _returnvalue_7 (Math|Conversions|ToFloat(Integer) _returnvalue_5))
  (bind _returnvalue_8 (Math|Conversions|ToFloat(Integer) _returnvalue_6))
  (bind _returnvalue_9 (Math|Vector|MakeVector 0.0 _returnvalue_8 _returnvalue_7))
  (bind _returnvalue_10 (+ _returnvalue_9 _offset_boite_de_nuit))
  (if (not (Variables|Default|GetModeMobat))
    (Transformation|SetActorLocation (Math|Vector|MakeVector (Math|Conversions|ToFloat(Integer) (Math|Integer|Clamp(Integer) (Math|Float|Truncate (.x (Transformation|GetActorLocation))) -13613 -13613)) (.y _returnvalue_10) (.z _returnvalue_10)) false false)))

(fn ConstructionScript)